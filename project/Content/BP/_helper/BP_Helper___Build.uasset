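; Helper Blueprint whose BuildHelper function sets up the helper HUD and an optional static camera view.
; It creates the BP_Helper___HUD widget, adds it to the viewport and prints a ready message in Korean.
; If the passed StaticCamera is valid, player 0's controller switches its view target to it.
; The function then returns the HUD to the caller.
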(fn BuildHelper
  (params (static_camera :type Camera%20Actor%20Object%20Reference))
  (Utilities|FlowControl|Sequence
    (:then_0
      ;[0.15 1 0.15 0.5] helper HUD 생성 및 설정
      (bind _returnvalue (UserInterface|CreateWidget "/Game/BP/_helper/BP_Helper___HUD.BP_Helper___HUD_C"))
      (bind _output_get (LocalVariables|Sethud _returnvalue))
      (UserInterface|Viewport|AddtoViewport _output_get 0)
      (Development|PrintString 0 "준비 완료"))
    (:then_1
      ;[0.15 1 0.15 0.5] Camera Setup
      (if (Utilities|IsValid static_camera)
        (Game|Player|SetViewTargetwithBlend (Game|GetPlayerController 0) static_camera 0.0 "VTBlend_Linear" 0.0 false)))
    (:then_2
      (return (LocalVariables|Gethud)))))